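; Trigger zone that turns off a linked Lightbulb when the player enters and lets them toggle it with F while inside.
; Begin overlap casts to BP_FirstPersonCharacter, hides the Lightbulb, sets the character's LightOff flag and enables input on player controller 0.
; F drives a FlipFlop that alternates the bulb's visibility and that flag.
; End overlap disables input without changing the light.
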(event Collision|EventActorEndOverlap
  (params (OtherActor :type Actor%20Object%20Reference))
  ;[0.15 0.15 0.15 0.5] When an object stops overlapping this Actor, check to see if it is the Player, if it is, disable input from them.
  (Utilities|Casting|CastToBP_FirstPersonCharacter OtherActor) ; Check if an object is of a certain class.
  (Input|DisableInput (Game|GetPlayerController 0)) ; Stop listening for input on this Actor on a specific Player Controller.
)

(event Collision|EventActorBeginOverlap
  (params (OtherActor :type Actor%20Object%20Reference))
  ;[0.15 0.15 0.15 0.5] Whenever something intersects with our Box collider component, check to see if it's the player, if it is, set the Light Off? Boolean to true, turn off the light, then Enable Input on PlayerController(0) so this Actor can receive input from the keyboard.
  (bind _asbp_first_person_character (Utilities|Casting|CastToBP_FirstPersonCharacter OtherActor)) ; Checks to see if an object is of a specific class.
  (Variables|/Game/FirstPerson/Blueprints/BP_FirstPersonCharacter.BP_FirstPersonCharacter_C|SetLight%20Off? _asbp_first_person_character true) ; Sets a Boolean to T or F.
  (Rendering|SetActorHiddenInGame (Variables|Default|GetLightbulb) true) ; Make a given Actor hidden or visible.
  (Input|EnableInput (Game|GetPlayerController 0)) ; Allows input from this Actor to be received by the given Player Controller.
)

(event Input|KeyboardEvents|F
  (params (Key :type Key%20Structure))
  (bind _lightbulb (Variables|Default|GetLightbulb))
  ;[0.15 0.15 0.15 0.5] When the F key is pressed, alternate between turning the light on or off, and setting the Player's Light Off? Boolean to T or F.
  (:Pressed
    (Utilities|FlowControl|FlipFlop ; Alternates between A and B output.
      (:A
        (Rendering|SetActorHiddenInGame _lightbulb false) ; Make a given Actor hidden or visible.
        (Variables|/Game/FirstPerson/Blueprints/BP_FirstPersonCharacter.BP_FirstPersonCharacter_C|SetLight%20Off? (stale Collision|EventActorBeginOverlap _asbp_first_person_character) false) ; Set a boolean to T or F.
      )
      (:B
        (Rendering|SetActorHiddenInGame _lightbulb true) ; Make a given Actor hidden or visible.
        (Variables|/Game/FirstPerson/Blueprints/BP_FirstPersonCharacter.BP_FirstPersonCharacter_C|SetLight%20Off? (stale Collision|EventActorBeginOverlap _asbp_first_person_character) true) ; Set a boolean to T or F.
      ))))

(fn ConstructionScript)