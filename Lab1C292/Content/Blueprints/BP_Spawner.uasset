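; BP_Spawner scatters pickups and other actors across level spawn points.
; On BeginPlay it gathers TargetPoints tagged SpawnPoint, spawns one BP_Pickup_Child_Unique at a random one, then gives each remaining point a 70% chance of a random ObjectsToSpawn class.
; The removed index re-evaluates Random, so it can differ from the unique pickup's point.
; Separate custom events spawn BP_Pickup at one or all SpawnPositions, or BP_Cube at the spawner.
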(event Custom|Spawn%20Thing
  ;[0.15 0.15 0.15 0.5] Spawn a BP_Cube at the location the Spawner is in the world.
  (Game|SpawnActorfromClass "/Game/Blueprints/BP_Cube.BP_Cube_C" (Math|Conversions|ToTransform(Vector) (Transformation|GetWorldLocation (Variables|Default|GetDefaultSceneRoot))) "Undefined" "MultiplyWithRoot" 0 0) ; Spawns an actor of the given class at the given location in the world.
)

(event Custom|Spawn%20at%20All%20Points
  ;[0.15 0.15 0.15 0.5] Go through every Actor in the array, then spawn an instance of the given class at the location of the Actor from the array.
  (for _array_element (Variables|Default|GetSpawn%20Positions)
    (Game|SpawnActorfromClass "/Game/Blueprints/BP_Pickup.BP_Pickup_C" (Transformation|GetActorTransform _array_element) "Undefined" "MultiplyWithRoot" 0 0)))

(event Custom|Spawn%20at%20Single%20Random%20Point
  ;[0.15 0.15 0.15 0.5] Randomly pick an item from the array, and then spawn the specified actor in the location of the randomly chosen item from the array.
  (Game|SpawnActorfromClass "/Game/Blueprints/BP_Pickup.BP_Pickup_C" (Transformation|GetActorTransform (Utilities|Array|Get(acopy) (Variables|Default|GetSpawn%20Positions) (Math|Random|RandomIntegerinRange 0 (- (Utilities|Array|Length (Variables|Default|GetSpawn%20Positions)) 1)))) "Undefined" "MultiplyWithRoot" 0 0))

(event EventBeginPlay
  ;[0.15 0.15 0.15 0.5] Make sure a specific object spawns one single time at a random location, remove that location from the spawnpoints array, then for each location in the array, randomly determine (70% chance) if something will spawn or not, if it does, then randomly pick an object to spawn from the Actor array.
  (bind _outactors (Actor|GetAllActorsOfClasswithTag "/Script/Engine.TargetPoint" "SpawnPoint"))
  (bind _output_get (Variables|Default|SetRuntime%20Array _outactors))
  (Game|SpawnActorfromClass "/Game/Blueprints/BP_Pickup_Child_Unique.BP_Pickup_Child_Unique_C" (Transformation|GetActorTransform (.OutItem (Utilities|Array|Random _output_get))) "Undefined" "MultiplyWithRoot" 0 0)
  (Utilities|Array|RemoveIndex (Variables|Default|GetRuntime%20Array) (.OutIndex (Utilities|Array|Random _output_get)))
  (for _array_element (Variables|Default|GetRuntime%20Array)
    (if (>= (Math|Random|RandomFloat) 0.3)
      (Game|SpawnActorfromClass (.OutItem (Utilities|Array|Random (Variables|Default|GetObjects%20to%20Spawn))) (Transformation|GetActorTransform _array_element) "Undefined" "MultiplyWithRoot" 0 0))))

(fn ConstructionScript)