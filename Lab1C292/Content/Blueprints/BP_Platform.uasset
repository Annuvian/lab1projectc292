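; BP_Platform is a player-operated moving platform that requires at least 3 collectables to use.
; Overlap with the first-person character stores a player reference and enables input, which is disabled when the overlap ends.
; Pressing F alternates a FlipFlop between playing and reversing a Timeline that lerps the cube from its BeginPlay position to a sideways, raised offset.
; When the Timeline finishes, the point light turns green at the start or red at the far end.
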(event Collision|EventActorBeginOverlap
  (params (OtherActor :type Actor%20Object%20Reference))
  ;[0.15 0.15 0.15 0.5] When an object starts overlapping the platform, check to see if it's the player, if it is, save them as a variable for easy reference later, then Enable Input. When something stops overlapping, check if it's the player, if it is, Disable Input.
  (bind _asbp_first_person_character (Utilities|Casting|CastToBP_FirstPersonCharacter OtherActor))
  (Variables|Default|SetOverlapping%20Player _asbp_first_person_character)
  (Input|EnableInput (Game|GetPlayerController 0)))

(event Collision|EventActorEndOverlap
  (params (OtherActor :type Actor%20Object%20Reference))
  ;[0.15 0.15 0.15 0.5] When an object starts overlapping the platform, check to see if it's the player, if it is, save them as a variable for easy reference later, then Enable Input. When something stops overlapping, check if it's the player, if it is, Disable Input.
  (Utilities|Casting|CastToBP_FirstPersonCharacter OtherActor)
  (Input|DisableInput (Game|GetPlayerController 0)))

(event EventBeginPlay
  ;[0.15 0.15 0.15 0.5] Get and save the starting position of the platform
  (Variables|Default|SetStart%20Pos (Transformation|GetWorldLocation (Variables|Default|GetCube))))

(event Input|KeyboardEvents|F
  (params (Key :type Key%20Structure))
  (bind _start_pos (Variables|Default|GetStart%20Pos))
  (bind _pointlight (Variables|Default|GetPointLight))
  ;[0.15 0.15 0.15 0.5] When the Player presses the F key (if input has been enabled for this Actor), check to make sure they have at least 3 collectables, and then alternate between playing or reversing the Timeline used for movement. Check to see if the Timeline delta is equal to A or B, if it is, set the light to green or red respectively.
  (:Pressed
    (if (>= (Variables|/Game/FirstPerson/Blueprints/BP_FirstPersonCharacter.BP_FirstPersonCharacter_C|GetCollected (Variables|Default|GetOverlapping%20Player)) 3)
      (Utilities|FlowControl|FlipFlop
        (:A
          (bind _movement_delta (Timeline|Movement Play)
            (:Update
              (Transformation|SetWorldLocation (Variables|Default|GetCube) (Math|Vector|Lerp(Vector) (Variables|Default|GetStart%20Pos) (Math|Vector|MakeVector (.x _start_pos) (+ (.y _start_pos) 5e+02) (+ (.z _start_pos) 3e+02)) _movement_delta) false false))
            (:Finished
              (if (== _movement_delta 0.0)
                (Rendering|Components|Light|SetLightColor _pointlight "(R=0.000000,G=1.000000,B=0.000000,A=1.000000)" true)
                (elif (== _movement_delta 1.0)
                  (Rendering|Components|Light|SetLightColor _pointlight "(R=1.000000,G=0.000000,B=0.000000,A=1.000000)" true))))))
        (:B
          (Timeline|Movement Reverse))))))

(fn ConstructionScript)