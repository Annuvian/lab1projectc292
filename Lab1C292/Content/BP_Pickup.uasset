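; BP_Pickup is a collectable that calls AddToCollection on the first-person player character when overlapped, then destroys itself.
; Overlaps from actors that fail the cast to BP_FirstPersonCharacter are ignored.
; On BeginPlay it stores the Cube's world location and plays BounceTimeline.
; The timeline's Bounce value lerps the Cube's transform, raising, rotating and scaling it to make the pickup stand out.
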(event EventBeginPlay
  ;[0.15 0.15 0.15 0.5] Just a fun way to animate the collectable bouncing and spinning to make it more obvious to the player that it's a collectable.
  (Variables|Default|SetStart%20Position (Transformation|GetWorldLocation (Variables|Default|GetCube)))
  (bind _bounce (Timeline|Bounce%20Timeline Play)
    (:Update
      (Transformation|SetWorldTransform (Variables|Default|GetCube) (Math|Transform|Lerp(Transform) (Math|Transform|MakeTransform (Variables|Default|GetStart%20Position) "0, 0, 0" "0.250000,0.250000,0.250000") (Math|Transform|MakeTransform (Math|Vector|MakeVector (.x (Variables|Default|GetStart%20Position)) (.y (Variables|Default|GetStart%20Position)) (+ (.z (Variables|Default|GetStart%20Position)) 1e+02)) "0.000000,180.000000,0.000000" "0.750000,0.750000,0.750000") _bounce) false false))))

(event Collision|EventActorBeginOverlap
  (params (OtherActor :type Actor%20Object%20Reference))
  ;[0.15 0.15 0.15 0.5] When something overlaps with the collectable, check if it's the player, if it is, call the Add to Collection method on the Player, then destroy the collectable.
  (bind _asbp_first_person_character (Utilities|Casting|CastToBP_FirstPersonCharacter OtherActor))
  (Default|AddtoCollection _asbp_first_person_character)
  (Actor|DestroyActor))

(fn ConstructionScript)