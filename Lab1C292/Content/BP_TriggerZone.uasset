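; Trigger zone actor that switches a referenced Lightbulb actor off when the first-person character enters and allows toggling it from inside.
; Begin overlap hides the bulb, sets the character's LightOff flag and enables player input on the zone.
; The F key runs a FlipFlop alternating bulb visibility and LightOff, with state independent of the forced switch-off on entry.
; End overlap by the character disables that input.
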(event Collision|EventActorEndOverlap
  (params (OtherActor :type Actor%20Object%20Reference))
  (Utilities|Casting|CastToBP_FirstPersonCharacter OtherActor)
  (Input|DisableInput (Game|GetPlayerController 0)))

(event Collision|EventActorBeginOverlap
  (params (OtherActor :type Actor%20Object%20Reference))
  ;[0.15 0.15 0.15 0.5] Whenever something intersects with our Box collider component, set the Lightbulb to be hidden in the game, effectively shutting off the light.
  (bind _asbp_first_person_character (Utilities|Casting|CastToBP_FirstPersonCharacter OtherActor))
  (Variables|/Game/FirstPerson/Blueprints/BP_FirstPersonCharacter.BP_FirstPersonCharacter_C|SetLight%20Off? _asbp_first_person_character true)
  (Rendering|SetActorHiddenInGame (Variables|Default|GetLightbulb) true) ; Make a given Actor hidden or visible.
  (Input|EnableInput (Game|GetPlayerController 0)))

(event Input|KeyboardEvents|F
  (params (Key :type Key%20Structure :default "None"))
  (:Pressed
    (Utilities|FlowControl|FlipFlop
      (:A
        (Rendering|SetActorHiddenInGame (Variables|Default|GetLightbulb) false) ; Make a given Actor hidden or visible.
        (Variables|/Game/FirstPerson/Blueprints/BP_FirstPersonCharacter.BP_FirstPersonCharacter_C|SetLight%20Off? (stale Collision|EventActorBeginOverlap _asbp_first_person_character) false))
      (:B
        (Rendering|SetActorHiddenInGame (Variables|Default|GetLightbulb) true) ; Make a given Actor hidden or visible.
        (Variables|/Game/FirstPerson/Blueprints/BP_FirstPersonCharacter.BP_FirstPersonCharacter_C|SetLight%20Off? (stale Collision|EventActorBeginOverlap _asbp_first_person_character) true)))))

(fn ConstructionScript)